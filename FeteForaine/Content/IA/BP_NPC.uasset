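; NPC Blueprint that patrols a set of locations and waves at the player on sight.
; RandomRoam moves through four PatrolLocation entries in sequence via AIMoveTo, pausing randomly after each arrival, and does nothing while IsWaving.
; PawnSensing sends the NPC toward a Player-tagged pawn, playing the wave as movement starts and resuming roaming five seconds later.
; Any sighting also triggers a retriggerable one-second delay before calling RandomRoam.
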(event OnSeePawn(PawnSensing)
  (params (Pawn :type Pawn%20Object%20Reference))
  (Utilities|FlowControl|Sequence
    (:then_0
      (if (Actor|ActorHasTag Pawn "Player")
        (AI|AIMoveTo self "0, 0, 0" Pawn 5.0 false
          (:then
            (Components|Animation|PlayAnimation (Variables|Character|GetMesh) "/Game/IA/Animation_Waving.Animation_Waving" false)
            (Variables|Default|SetIsWaving true)
            (Utilities|FlowControl|Delay 5.0)
            (Variables|Default|SetIsWaving false)
            (Components|Animation|PlayAnimation (Variables|Character|GetMesh) "/Game/Characters/Mannequins/Animations/Manny/MM_Walk_Fwd.MM_Walk_Fwd" false)
            (CallFunction|RandomRoam)))))
    (:then_1
      (Utilities|FlowControl|RetriggerableDelay 1.0)
      (CallFunction|RandomRoam))))

(event Custom|Random%20roam
  (if (not (Variables|Default|GetIsWaving))
    (AI|AIMoveTo self (Utilities|Array|Get(acopy) (Variables|Default|GetPatrolLocation) (Variables|Default|GetLocations)) 0 5.0 false
      (:OnSuccess
        (Utilities|FlowControl|Delay (Math|Random|RandomFloatinRange 1.0 3.0))
        (CallFunction|RandomRoam)
        (Math|Integer|IncrementInt (Variables|Default|GetLocations)
          (:%20%20
            (if (== (Variables|Default|GetLocations) 4)
              (Variables|Default|SetLocations 0))))))))

(event EventBeginPlay
  (CallFunction|RandomRoam))

(fn ConstructionScript)