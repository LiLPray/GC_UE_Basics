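; BP_TriggerBoxAuto is a trigger for the bumper car (auto-tamponeuse) area that moves player control from the character to a car.
; When a BP_ThirdPersonCharacter begins overlapping, it adds the IMC_Auto mapping context and player controller 0 possesses a random BP_Auto in the level.
; When the character stops overlapping, it calls Reinitialisation on every BP_Auto.
; An unconnected branch that counts "Cylindre"-tagged actors never runs.
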(event Collision|EventActorBeginOverlap
  (params (OtherActor :type Actor%20Object%20Reference))
  (bind _asbp_third_person_character (Utilities|Casting|CastToBP_ThirdPersonCharacter OtherActor))
  (if (Utilities|IsValid _asbp_third_person_character)
    (Input|AddMappingContext (PlayerController|LocalPlayerSubsystems|GetEnhancedInputLocalPlayerSubsystem (Game|GetPlayerController 0)) "/Game/Auto-tamponeuse/IMC_Auto.IMC_Auto" 0 "(bIgnoreAllPressedKeysUntilRelease=True,bForceImmediately=False,bNotifyUserSettings=False)")
    (bind _outactors (Actor|GetAllActorsOfClass "/Game/Auto-tamponeuse/BP_Auto.BP_Auto_C"))
    (Pawn|Possess (Game|GetPlayerController 0) (.OutItem (Utilities|Array|Random _outactors)))))

(event Collision|EventActorEndOverlap
  (params (OtherActor :type Actor%20Object%20Reference))
  (bind _asbp_third_person_character (Utilities|Casting|CastToBP_ThirdPersonCharacter OtherActor))
  (if (Utilities|IsValid _asbp_third_person_character)
    (bind _outactors (Actor|GetAllActorsOfClass "/Game/Auto-tamponeuse/BP_Auto.BP_Auto_C"))
    (for _array_element _outactors
      (bind _asbp_auto (Utilities|Casting|CastToBP_Auto _array_element))
      (Default|Reinitialisation _asbp_auto))))

(fn ConstructionScript)