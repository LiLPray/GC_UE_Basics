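; BP_Auto is a drivable bumper car moved by Enhanced Input actions.
; IA_MoveAuto applies a physics force to its static mesh along the right vector, scaled by the input value and MoveForce.
; IA_TurnAuto only resets the mesh to zero world rotation, as the yaw calculation using TurnForce is left unconnected.
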(event Input|EnhancedActionEvents|EnhancedInputActionIA_MoveAuto
  (params (ActionValue :type Float%20%28double-precision%29) (ElapsedSeconds :type Float%20%28double-precision%29) (TriggeredSeconds :type Float%20%28double-precision%29) (InputAction :type Input%20Action%20Object%20Reference :default "/Game/Auto-tamponeuse/IA_MoveAuto.IA_MoveAuto"))
  (Physics|AddForce (Variables|Default|GetStaticMesh) (* (* ActionValue (Variables|Default|GetMoveForce)) (Math|Vector|GetRightVector (Variables|Default|GetStaticMesh))) "None" false))

(event Input|EnhancedActionEvents|EnhancedInputActionIA_TurnAuto
  (params (ActionValue :type Float%20%28double-precision%29) (ElapsedSeconds :type Float%20%28double-precision%29) (TriggeredSeconds :type Float%20%28double-precision%29) (InputAction :type Input%20Action%20Object%20Reference :default "/Game/Auto-tamponeuse/IA_TurnAuto.IA_TurnAuto"))
  (Transformation|SetWorldRotation (Variables|Default|GetStaticMesh) "0, 0, 0" false false))

(fn ConstructionScript)